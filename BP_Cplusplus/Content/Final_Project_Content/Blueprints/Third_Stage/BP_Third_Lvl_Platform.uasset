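; BP_Third_Lvl_Platform is a third-stage level platform that moves once the stage boss is dead.
; It records its starting location on BeginPlay, then every Tick finds the first actor from an all-actors-of-class query and casts it to Third_Stage_Boss.
; While that boss's Dead flag is set, it plays a timeline whose track is added to the start location to reposition the platform without sweeping.
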(event EventTick
  (params (DeltaSeconds :type Float%20%28single-precision%29))
  (bind _outactors (Actor|GetAllActorsOfClass 0))
  (bind _asthird_stage_boss (Utilities|Casting|CastToThird_Stage_Boss (Utilities|Array|Get(acopy) _outactors)))
  (if (Variables|/Game/Final_Project_Content/Blueprints/Third_Stage/Third_Stage_Boss.Third_Stage_Boss_C|GetDead _asthird_stage_boss)
    (bind _newtrack_0 (Timeline|Timeline_0 Play)
      (:Update
        (Transformation|SetActorLocation (+ _newtrack_0 (Variables|Default|GetLocation)) false false)))))

(event EventBeginPlay
  (Variables|Default|SetLocation (Transformation|GetActorLocation)))

(fn ConstructionScript)