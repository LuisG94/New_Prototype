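; BP_PlayerAmmo is the player's ammo actor, which damages enemies and the third-stage boss on overlap, then destroys itself.
; Six capsule overlap events each cast to one enemy class and call its damage function with fixed damage.
; The turret branch intends bonus head damage, but compares the ammo's own overlapped capsule to the turret's head collision, so body damage applies.
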(event OnComponentBeginOverlap(Capsule1)
  (params (OverlappedComponent :type Primitive%20Component%20Object%20Reference) (OtherActor :type Actor%20Object%20Reference) (OtherComp :type Primitive%20Component%20Object%20Reference) (OtherBodyIndex :type Integer) (bFromSweep :type Boolean) (SweepResult :type Hit%20Result%20Structure%20%28by%20ref%29))
  (bind _asbp_enemy_eye_00 (Utilities|Casting|CastToBP_Enemy_Eye00 OtherActor))
  (Default|DMGEnemy _asbp_enemy_eye_00 45.0)
  (Actor|DestroyActor))

(event OnComponentBeginOverlap(Capsule)
  (params (OverlappedComponent :type Primitive%20Component%20Object%20Reference) (OtherActor :type Actor%20Object%20Reference) (OtherComp :type Primitive%20Component%20Object%20Reference) (OtherBodyIndex :type Integer) (bFromSweep :type Boolean) (SweepResult :type Hit%20Result%20Structure%20%28by%20ref%29))
  (bind _asbp_enemy_eye_1 (Utilities|Casting|CastToBP_Enemy_Eye1 OtherActor))
  (Default|DMGEnemy _asbp_enemy_eye_1 34.0)
  (Actor|DestroyActor))

(event OnComponentBeginOverlap(Capsule2)
  (params (OverlappedComponent :type Primitive%20Component%20Object%20Reference) (OtherActor :type Actor%20Object%20Reference) (OtherComp :type Primitive%20Component%20Object%20Reference) (OtherBodyIndex :type Integer) (bFromSweep :type Boolean) (SweepResult :type Hit%20Result%20Structure%20%28by%20ref%29))
  (bind _asbp_enemy_eye_2 (Utilities|Casting|CastToBP_Enemy_Eye2 OtherActor))
  (Default|DMGEnemy _asbp_enemy_eye_2 35.0)
  (Actor|DestroyActor))

(event OnComponentBeginOverlap(Capsule3)
  (params (OverlappedComponent :type Primitive%20Component%20Object%20Reference) (OtherActor :type Actor%20Object%20Reference) (OtherComp :type Primitive%20Component%20Object%20Reference) (OtherBodyIndex :type Integer) (bFromSweep :type Boolean) (SweepResult :type Hit%20Result%20Structure%20%28by%20ref%29))
  (bind _asthird_stage_boss (Utilities|Casting|CastToThird_Stage_Boss OtherActor))
  (Default|DamageThirdBoss _asthird_stage_boss 8.0)
  (Actor|DestroyActor))

(event OnComponentBeginOverlap(Capsule4)
  (params (OverlappedComponent :type Primitive%20Component%20Object%20Reference) (OtherActor :type Actor%20Object%20Reference) (OtherComp :type Primitive%20Component%20Object%20Reference) (OtherBodyIndex :type Integer) (bFromSweep :type Boolean) (SweepResult :type Hit%20Result%20Structure%20%28by%20ref%29))
  (bind _asbp_turret_enemy (Utilities|Casting|CastToBP_Turret_Enemy OtherActor))
  (if (== OverlappedComponent (Variables|/Game/Final_Project_Content/Blueprints/Enemies/BP_Turret_Enemy.BP_Turret_Enemy_C|GetHead_Turret_Collision _asbp_turret_enemy))
    (Default|DMGTurretEnemy _asbp_turret_enemy 7e+01)
    (Actor|DestroyActor)
    (else
      (Default|DMGTurretEnemy _asbp_turret_enemy 3e+01)
      (Actor|DestroyActor))))

(event OnComponentBeginOverlap(Capsule5)
  (params (OverlappedComponent :type Primitive%20Component%20Object%20Reference) (OtherActor :type Actor%20Object%20Reference) (OtherComp :type Primitive%20Component%20Object%20Reference) (OtherBodyIndex :type Integer) (bFromSweep :type Boolean) (SweepResult :type Hit%20Result%20Structure%20%28by%20ref%29))
  (bind _asbp_gun_enemy (Utilities|Casting|CastToBP_Gun_Enemy OtherActor))
  (Default|DMGGunEnemy _asbp_gun_enemy 45.0)
  (Actor|DestroyActor))

(event EventBeginPlay)

(event Collision|EventActorBeginOverlap
  (params (OtherActor :type Actor%20Object%20Reference)))

(event EventTick
  (params (DeltaSeconds :type Float%20%28single-precision%29)))

(fn ConstructionScript)