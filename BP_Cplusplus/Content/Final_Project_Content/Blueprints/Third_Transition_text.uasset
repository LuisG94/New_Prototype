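; Trigger actor that plays the third transition's on-screen text when the 2D side-scroller character enters its box.
; On overlap it disables the player's input, then shows two text widgets in sequence, each removed after a short delay.
; Input is re-enabled after the second widget is removed, and no guard prevents the sequence from replaying on re-entry.
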(event OnComponentBeginOverlap(Box)
  (params (OverlappedComponent :type Primitive%20Component%20Object%20Reference) (OtherActor :type Actor%20Object%20Reference) (OtherComp :type Primitive%20Component%20Object%20Reference) (OtherBodyIndex :type Integer) (bFromSweep :type Boolean) (SweepResult :type Hit%20Result%20Structure%20%28by%20ref%29))
  (bind _as2dside_scroller_character_0 (Utilities|Casting|CastTo2DSideScrollerCharacter0 OtherActor))
  (Input|DisableInput _as2dside_scroller_character_0 0)
  (bind _returnvalue (UserInterface|CreateWidget "/Game/Final_Project_Content/Widgets/Third_Transition_text2.Third_Transition_text2_C"))
  (UserInterface|Viewport|AddtoViewport _returnvalue 0)
  (Utilities|FlowControl|Delay 1.6)
  (Widget|RemovefromParent _returnvalue)
  (bind _returnvalue_2 (UserInterface|CreateWidget "/Game/Final_Project_Content/Widgets/Third_Transition_text3.Third_Transition_text3_C"))
  (UserInterface|Viewport|AddtoViewport _returnvalue_2 0)
  (Utilities|FlowControl|Delay 1.6)
  (Widget|RemovefromParent _returnvalue_2)
  (Input|EnableInput _as2dside_scroller_character_0 0))

(event EventBeginPlay)

(event Collision|EventActorBeginOverlap
  (params (OtherActor :type Actor%20Object%20Reference)))

(event EventTick
  (params (DeltaSeconds :type Float%20%28single-precision%29)))

(fn ConstructionScript)