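; BP_2nd_Boss_Guard3 is a moving, shooting guard for the third stage's second boss stage.
; A custom attack event spawns BP_Boss_Ammo at its arrow, throttled by a DoOnce that resets after 1.5 seconds.
; Tick plays a timeline that offsets the actor from its starting location.
; A damage event drains health, then at zero flags it dead, destroys its arrow, box and sprite components, and plays an explosion sound.
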(event Custom|damage
  (params (DMG%20In :type Float%20%28single-precision%29))
  ;[1 1 1] damage guard
  (bind _output_get (Variables|Default|SetSecond_Stage_Guard_Health (- (Variables|Default|GetSecond_Stage_Guard_Health) DMG%20In)))
  (if (<= _output_get 0.0)
    (Variables|Default|SetDead true)
    (Utilities|FlowControl|Sequence
      (:then_0
        (Components|DestroyComponent (Variables|Default|GetFirst_Arrow)))
      (:then_1
        (Components|DestroyComponent (Variables|Default|GetFirst_Box)))
      (:then_2
        (Components|DestroyComponent (Variables|Default|GetFirst_PaperSprite)))
      (:then_3
        (Audio|PlaySound2D "/Game/Final_Project_Content/Sound_Music/SoundsCrate-SciFi-Explosion5__1_.SoundsCrate-SciFi-Explosion5__1_" 1.0 1.0 0.0 0 0)))))

(event Custom|3rd_Second_Stage_Guard_Attk
  ;[1 1 1] Guard attk
  (Utilities|FlowControl|DoOnce false :!label _label
    (:Completed
      (Game|SpawnActorfromClass "/Game/Final_Project_Content/Blueprints/Attacks/BP_Boss_Ammo.BP_Boss_Ammo_C" (Transformation|GetWorldTransform (Variables|Default|GetFirst_Arrow)) "Undefined" 0 0)
      (Utilities|FlowControl|Delay 1.5)
      (goto _label Reset))))

(event EventTick
  (params (DeltaSeconds :type Float%20%28single-precision%29))
  (if true
    (bind _newtrack_0 (Timeline|Timeline_0 Play)
      (:Update
        (Transformation|SetActorLocation (+ _newtrack_0 (Variables|Default|Getlocation)) false false)))))

(event EventBeginPlay
  (Variables|Default|Setlocation (Transformation|GetActorLocation))
  (Utilities|FlowControl|Delay 0.2)
  (Variables|Default|SetStart%20Moving true))

(fn ConstructionScript)