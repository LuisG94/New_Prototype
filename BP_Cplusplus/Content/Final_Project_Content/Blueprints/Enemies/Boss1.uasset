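; Boss enemy with a Paper2D sprite that turns to face the player, shoots and dies when its health runs out.
; Tick sets yaw toward the player and fires BP_Ammo1 from an arrow, throttled to 1.5 seconds, when the signed X-axis distance is at most 300.
; A range check re-applies the boss's current location, so it adds no movement.
; DMGBOSS handles damage, and BeginPlay adds the Boss_Health widget.
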(event Custom|DMG%20BOSS
  (params (DMG%20In :type Float%20%28single-precision%29))
  ;[1 1 1] damageboss
  (bind _output_get (Variables|Default|SetBOSS%20Health (- (Variables|Default|GetBOSS%20Health) DMG%20In)))
  (if (<= _output_get 0.0)
    (Actor|DestroyActor)))

(event Custom|BOSSAtck
  ;[1 1 1] Boss Attack
  (Utilities|FlowControl|DoOnce false :!label _label
    (:Completed
      (Game|SpawnActorfromClass "/Game/Final_Project_Content/Blueprints/Attacks/BP_Ammo1.BP_Ammo1_C" (Transformation|GetWorldTransform (Variables|Default|GetArrow)) "Undefined" 0 0)
      (Utilities|FlowControl|Delay 1.5)
      (goto _label Reset))))

(event EventTick
  (params (DeltaSeconds :type Float%20%28single-precision%29))
  (bind _returnvalue (Transformation|GetActorLocation))
  (Utilities|FlowControl|Sequence
    (:then_0
      (Transformation|SetActorRotation (Math|Rotator|MakeRotator 0.0 0.0 (.yaw (Math|Rotator|FindLookatRotation (Transformation|GetActorLocation) (Transformation|GetActorLocation (Game|GetPlayerCharacter 0)))))))
    (:then_1
      (bind _output_get (Variables|Default|SetDistance (- (.x (Transformation|GetActorLocation (Game|GetPlayerController 0))) (.x (Transformation|GetWorldLocation (Variables|Default|GetPaperSprite))))))
      (if (<= _output_get 3e+02)
        (CallFunction|BOSSAtck)))
    (:then_2
      (Variables|Default|SetActorX (.x _returnvalue)))
    (:then_3
      (Variables|Default|SetActorY (.y _returnvalue)))
    (:then_4
      (Variables|Default|SetActorZ (.z _returnvalue)))
    (:then_5
      (if (Math|Float|InRange(Float) (Variables|Default|GetDistance) 0.0 4e+02)
        (Transformation|SetActorLocation (Math|Vector|MakeVector (Variables|Default|GetActorX) (Variables|Default|GetActorY) (Variables|Default|GetActorZ)) false false)))))

(event EventBeginPlay
  ;[1 1 1] Health Bar
  (Class|ActorComponent|SetIsReplicated (Variables|Default|GetPaperSprite) true)
  (bind _returnvalue (UserInterface|CreateWidget "/Game/Final_Project_Content/Widgets/Boss_Health.Boss_Health_C"))
  (UserInterface|Viewport|AddtoViewport _returnvalue 0))

(fn ConstructionScript)