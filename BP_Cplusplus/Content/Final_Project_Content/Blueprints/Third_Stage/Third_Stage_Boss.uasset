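; Third-stage boss for a 2D Paper2D level, with a health widget, damage flash and death cleanup.
; Tick polls health to run four phases, each teleporting the boss away, spawning four guards, and returning it once all are dead.
; It fires ammo when the player is within X range and, once hurt enough, tracks player height.
; At low health it adds a blast attack, with DoOnce-plus-Delay cooldowns pacing shots.
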(event Custom|Damage_Third_Boss
  (params (DMG%20In :type Float%20%28single-precision%29))
  ;[1 1 1] damageboss
  (bind _output_get (Variables|Default|SetThird_Boss_Health (- (Variables|Default|GetThird_Boss_Health) DMG%20In)))
  (if (<= _output_get 0.0)
    (Variables|Default|SetDead true)
    (Utilities|FlowControl|Sequence
      (:then_0
        (Components|DestroyComponent (Variables|Default|GetPaperFlipbook)))
      (:then_1
        (Components|DestroyComponent (Variables|Default|GetBox1)))
      (:then_2
        (Components|DestroyComponent (Variables|Default|GetBox)))
      (:then_3
        (Components|DestroyComponent (Variables|Default|GetArrow)))
      (:then_4
        (Components|DestroyComponent (Variables|Default|GetArrow1)))
      (:then_5
        (Audio|PlaySound2D "/Game/Final_Project_Content/Sound_Music/SoundsCrate-SciFi-Explosion5__1_.SoundsCrate-SciFi-Explosion5__1_" 1.0 1.0 0.0 0 0)))
    (else
      (Sprite|SetFlipbook (Variables|Default|GetPaperFlipbook) "/Game/Final_Project_Content/Sprites/Enemies/Boss_lowHP_Flipbook.Boss_lowHP_Flipbook")
      (Utilities|FlowControl|Delay 0.5)
      (Sprite|SetFlipbook (Variables|Default|GetPaperFlipbook) "/Game/Final_Project_Content/Sprites/Enemies/Boss_Chase2.Boss_Chase2"))))

(event Custom|second%20boss%20attack
  ;[1 1 1] second boss attack
  (Utilities|FlowControl|DoOnce false :!label _label
    (:Completed
      (Game|SpawnActorfromClass "/Game/Final_Project_Content/Blueprints/Attacks/BP_Boss_Ammo.BP_Boss_Ammo_C" (Transformation|GetWorldTransform (Variables|Default|GetArrow)) "Undefined" 0 0)
      (Utilities|FlowControl|Delay 0.5)
      (goto _label Reset))))

(event Custom|First_Boss_Stage
  ;[1 1 1] 1st. Boss will disappear and guard will appear
  (Transformation|SetActorLocation "-2215.000000, 0,676.000000" false false)
  (Game|SpawnActorfromClass "/Game/Final_Project_Content/Blueprints/Third_Stage/First_Boss_Stage/BP_1st_Boss_Guard1.BP_1st_Boss_Guard1_C" (Math|Transform|MakeTransform "851.000000, 0,708.000000") "Undefined" 0 0)
  (Game|SpawnActorfromClass "/Game/Final_Project_Content/Blueprints/Third_Stage/First_Boss_Stage/BP_1st_Boss_Guard2.BP_1st_Boss_Guard2_C" (Math|Transform|MakeTransform "851.000000, 0,642.000000") "Undefined" 0 0)
  (Game|SpawnActorfromClass "/Game/Final_Project_Content/Blueprints/Third_Stage/First_Boss_Stage/BP_1st_Boss_Guard3.BP_1st_Boss_Guard3_C" (Math|Transform|MakeTransform "851.000000, 0,576.000000") "Undefined" 0 0)
  (Game|SpawnActorfromClass "/Game/Final_Project_Content/Blueprints/Third_Stage/First_Boss_Stage/BP_1st_Boss_Guard4.BP_1st_Boss_Guard4_C" (Math|Transform|MakeTransform "851.000000, 0,511.000000") "Undefined" 0 0))

(event Custom|Second_Boss_Stage
  ;[1 1 1] 2nd. Boss will disapear and second guard will appear
  (Transformation|SetActorLocation "-2215.000000, 0,676.000000" false false)
  (Game|SpawnActorfromClass "/Game/Final_Project_Content/Blueprints/Third_Stage/Second_Boss_Stage/BP_2nd_Boss_Guard1.BP_2nd_Boss_Guard1_C" (Math|Transform|MakeTransform "436.000000, 0,736.000000") "Undefined" 0 0)
  (Game|SpawnActorfromClass "/Game/Final_Project_Content/Blueprints/Third_Stage/Second_Boss_Stage/BP_2nd_Boss_Guard2.BP_2nd_Boss_Guard2_C" (Math|Transform|MakeTransform "509.000000, 0,736.000000") "Undefined" 0 0)
  (Game|SpawnActorfromClass "/Game/Final_Project_Content/Blueprints/Third_Stage/Second_Boss_Stage/BP_2nd_Boss_Guard3.BP_2nd_Boss_Guard3_C" (Math|Transform|MakeTransform "582.000000, 0,736.000000") "Undefined" 0 0)
  (Game|SpawnActorfromClass "/Game/Final_Project_Content/Blueprints/Third_Stage/Second_Boss_Stage/BP_2nd_Boss_Guard4.BP_2nd_Boss_Guard4_C" (Math|Transform|MakeTransform "659.000000, 0,736.000000") "Undefined" 0 0))

(event Custom|Third_Boss_Stage
  ;[1 1 1] 3rd. boss will stay in place but guard will come up again
  (Transformation|SetActorLocation "-2215.000000, 0,676.000000" false false)
  (Utilities|FlowControl|DoOnce false
    (:Completed
      (Game|SpawnActorfromClass "/Game/Final_Project_Content/Blueprints/Third_Stage/Third_Boss_Stage/BP_3rd_Boss_Guard1.BP_3rd_Boss_Guard1_C" (Math|Transform|MakeTransform "894.000000, 0,636.000000") "Undefined" 0 0)
      (Utilities|FlowControl|DoOnce false
        (:Completed
          (Game|SpawnActorfromClass "/Game/Final_Project_Content/Blueprints/Third_Stage/Third_Boss_Stage/BP_3rd_Boss_Guard2.BP_3rd_Boss_Guard2_C" (Math|Transform|MakeTransform "851.000000, 0,585.000000") "Undefined" 0 0)
          (Utilities|FlowControl|DoOnce false
            (:Completed
              (Game|SpawnActorfromClass "/Game/Final_Project_Content/Blueprints/Third_Stage/Third_Boss_Stage/BP_3rd_Boss_Guard3.BP_3rd_Boss_Guard3_C" (Math|Transform|MakeTransform "895.000000, 0,542.000000") "Undefined" 0 0)
              (Utilities|FlowControl|DoOnce false
                (:Completed
                  (Game|SpawnActorfromClass "/Game/Final_Project_Content/Blueprints/Third_Stage/Third_Boss_Stage/BP_3rd_Boss_Guard4.BP_3rd_Boss_Guard4_C" (Math|Transform|MakeTransform "851.000000, 0,511.000000") "Undefined" 0 0))))))))))

(event Custom|Move_Up_Down
  (bind _returnvalue (Transformation|GetActorLocation))
  (bind _returnvalue_2 (Transformation|GetActorLocation))
  (bind (_x _y _z) (Math|Vector|BreakVector _returnvalue))
  (bind (_x_2 _y_2 _z_2) (Math|Vector|BreakVector _returnvalue_2))
  ;[1 1 1] follows player on the z axis
  (bind _output_get (Variables|Default|SetThird%20Boss%20Z%20Distance (- (.z (Transformation|GetActorLocation (Game|GetPlayerCharacter 0))) (.z (Transformation|GetWorldLocation (Variables|Default|GetPaperFlipbook))))))
  (if (> _output_get -1.4e+02)
    (Transformation|SetActorLocation (Math|Vector|MakeVector _x_2 _y_2 (+ _z_2 3.0)) false false)
    (else
      (Transformation|SetActorLocation (Math|Vector|MakeVector _x _y (- _z 3.0)) false false))))

(event Custom|Third_Boss_Atck
  ;[1 1 1] boss attack
  (Utilities|FlowControl|DoOnce false :!label _label
    (:Completed
      (Game|SpawnActorfromClass "/Game/Final_Project_Content/Blueprints/Attacks/BP_Boss_Ammo.BP_Boss_Ammo_C" (Transformation|GetWorldTransform (Variables|Default|GetArrow)) "Undefined" 0 0)
      (Utilities|FlowControl|Delay 0.7)
      (goto _label Reset))))

(event Custom|Last%20Boss%20Stage
  ;[1 1 1] 4th boss stage
  (Transformation|SetActorLocation "-2215.000000, 0,676.000000" false false)
  (Utilities|FlowControl|DoOnce false
    (:Completed
      (Game|SpawnActorfromClass "/Game/Final_Project_Content/Blueprints/Third_Stage/Fourth_Boss_Stage/BP_4th_Boss_Guard.BP_4th_Boss_Guard_C" (Math|Transform|MakeTransform "582.000000, 0,736.000000") "Undefined" 0 0)
      (Utilities|FlowControl|DoOnce false
        (:Completed
          (Game|SpawnActorfromClass "/Game/Final_Project_Content/Blueprints/Third_Stage/Fourth_Boss_Stage/BP_4th_Boss_Guard2.BP_4th_Boss_Guard2_C" (Math|Transform|MakeTransform "659.000000, 0,736.000000") "Undefined" 0 0)
          (Utilities|FlowControl|DoOnce false
            (:Completed
              (Game|SpawnActorfromClass "/Game/Final_Project_Content/Blueprints/Third_Stage/Fourth_Boss_Stage/BP_4th_Boss_Guard3.BP_4th_Boss_Guard3_C" (Math|Transform|MakeTransform "428.000000, 0,585.000000") "Undefined" 0 0)
              (Utilities|FlowControl|DoOnce false
                (:Completed
                  (Game|SpawnActorfromClass "/Game/Final_Project_Content/Blueprints/Third_Stage/Fourth_Boss_Stage/BP_4th_Boss_Guard4.BP_4th_Boss_Guard4_C" (Math|Transform|MakeTransform "780.000000, 0,581.000000") "Undefined" 0 0))))))))))

(event Custom|Last%20Attack
  ;[1 1 1] Comment
  (Utilities|FlowControl|DoOnce false :!label _label
    (:Completed
      (Game|SpawnActorfromClass "/Game/Final_Project_Content/Blueprints/Attacks/BP_Blast.BP_Blast_C" (Transformation|GetWorldTransform (Variables|Default|GetArrow1)) "Undefined" 0 0)
      (Utilities|FlowControl|Delay 0.2)
      (goto _label Reset))))

(event EventTick
  (params (DeltaSeconds :type Float%20%28single-precision%29))
  (if (== (Variables|Default|GetThird_Boss_Health) 1e+02)
    (Utilities|FlowControl|Delay 11.0)
    (else
      (Utilities|FlowControl|Sequence
        (:then_0
          ;[1 1 1] will attack when in range
          (bind _output_get (Variables|Default|SetThird_Boss_Distance (- (.x (Transformation|GetActorLocation (Game|GetPlayerController 0))) (.x (Transformation|GetWorldLocation (Variables|Default|GetPaperFlipbook))))))
          (if (<= _output_get 3e+02)
            (CallFunction|ThirdBossAtck)))
        (:then_1
          ;[1 1 1] Activate First Stage
          (if (<= (Variables|Default|GetThird_Boss_Health) 8e+01)
            (Utilities|FlowControl|DoOnce false
              (:Completed
                (CallFunction|FirstBossStage)))))
        (:then_2
          ;[1 1 1] reset boss to position once first guard is dead
          (Utilities|FlowControl|Sequence
            (:then_0
              (bind _outactors (Actor|GetAllActorsOfClass "/Game/Final_Project_Content/Blueprints/Third_Stage/First_Boss_Stage/BP_1st_Boss_Guard1.BP_1st_Boss_Guard1_C"))
              (bind _asbp_1st_boss_guard_1 (Utilities|Casting|CastToBP_1st_Boss_Guard1 (Utilities|Array|Get(acopy) _outactors)))
              (if (Math|Boolean|ANDBoolean (Variables|/Game/Final_Project_Content/Blueprints/Third_Stage/First_Boss_Stage/BP_1st_Boss_Guard1.BP_1st_Boss_Guard1_C|GetDead _asbp_1st_boss_guard_1) (Variables|/Game/Final_Project_Content/Blueprints/Third_Stage/First_Boss_Stage/BP_1st_Boss_Guard2.BP_1st_Boss_Guard2_C|GetDead (stale _asbp_1st_boss_guard_2)) (Variables|/Game/Final_Project_Content/Blueprints/Third_Stage/First_Boss_Stage/BP_1st_Boss_Guard3.BP_1st_Boss_Guard3_C|GetDead (stale _asbp_1st_boss_guard_3)) (Variables|/Game/Final_Project_Content/Blueprints/Third_Stage/First_Boss_Stage/BP_1st_Boss_Guard4.BP_1st_Boss_Guard4_C|GetDead (stale _asbp_1st_boss_guard_4)))
                (Utilities|FlowControl|DoOnce false
                  (:Completed
                    (Transformation|SetActorLocation "1020.000000, 0,632.000000" false false)))))
            (:then_1
              (bind _outactors_2 (Actor|GetAllActorsOfClass "/Game/Final_Project_Content/Blueprints/Third_Stage/First_Boss_Stage/BP_1st_Boss_Guard2.BP_1st_Boss_Guard2_C"))
              (bind _asbp_1st_boss_guard_2 (Utilities|Casting|CastToBP_1st_Boss_Guard2 (Utilities|Array|Get(acopy) _outactors_2))))
            (:then_2
              (bind _outactors_3 (Actor|GetAllActorsOfClass "/Game/Final_Project_Content/Blueprints/Third_Stage/First_Boss_Stage/BP_1st_Boss_Guard3.BP_1st_Boss_Guard3_C"))
              (bind _asbp_1st_boss_guard_3 (Utilities|Casting|CastToBP_1st_Boss_Guard3 (Utilities|Array|Get(acopy) _outactors_3))))
            (:then_3
              (bind _outactors_4 (Actor|GetAllActorsOfClass "/Game/Final_Project_Content/Blueprints/Third_Stage/First_Boss_Stage/BP_1st_Boss_Guard4.BP_1st_Boss_Guard4_C"))
              (bind _asbp_1st_boss_guard_4 (Utilities|Casting|CastToBP_1st_Boss_Guard4 (Utilities|Array|Get(acopy) _outactors_4))))))
        (:then_3
          ;[1 1 1] as long as health is between 75-50, boss will follow on z axis
          (if (<= (Variables|Default|GetThird_Boss_Health) 8e+01)
            (CallFunction|MoveUpDown)))
        (:then_4
          ;[1 1 1] Activate Second Boss Stage
          (if (and (<= (Variables|Default|GetThird_Boss_Health) 6e+01) (> (Variables|Default|GetThird_Boss_Health) 4e+01))
            (Utilities|FlowControl|DoOnce false
              (:Completed
                (CallFunction|SecondBossStage)))))
        (:then_5
          ;[1 1 1] reset boss position after second guard is dead
          (Utilities|FlowControl|Sequence
            (:then_0
              (bind _outactors_5 (Actor|GetAllActorsOfClass "/Game/Final_Project_Content/Blueprints/Third_Stage/Second_Boss_Stage/BP_2nd_Boss_Guard1.BP_2nd_Boss_Guard1_C"))
              (bind _asbp_2nd_boss_guard_1 (Utilities|Casting|CastToBP_2nd_Boss_Guard1 (Utilities|Array|Get(acopy) _outactors_5)))
              (if (Math|Boolean|ANDBoolean (Variables|/Game/Final_Project_Content/Blueprints/Third_Stage/Second_Boss_Stage/BP_2nd_Boss_Guard1.BP_2nd_Boss_Guard1_C|GetDead _asbp_2nd_boss_guard_1) (Variables|/Game/Final_Project_Content/Blueprints/Third_Stage/Second_Boss_Stage/BP_2nd_Boss_Guard2.BP_2nd_Boss_Guard2_C|GetDead (stale _asbp_2nd_boss_guard_2)) (Variables|/Game/Final_Project_Content/Blueprints/Third_Stage/Second_Boss_Stage/BP_2nd_Boss_Guard3.BP_2nd_Boss_Guard3_C|GetDead (stale _asbp_2nd_boss_guard_3)) (Variables|/Game/Final_Project_Content/Blueprints/Third_Stage/Second_Boss_Stage/BP_2nd_Boss_Guard4.BP_2nd_Boss_Guard4_C|GetDead (stale _asbp_2nd_boss_guard_4)))
                (Utilities|FlowControl|DoOnce false
                  (:Completed
                    (Transformation|SetActorLocation "1020.000000, 0,632.000000" false false)))))
            (:then_1
              (bind _outactors_6 (Actor|GetAllActorsOfClass "/Game/Final_Project_Content/Blueprints/Third_Stage/Second_Boss_Stage/BP_2nd_Boss_Guard2.BP_2nd_Boss_Guard2_C"))
              (bind _asbp_2nd_boss_guard_2 (Utilities|Casting|CastToBP_2nd_Boss_Guard2 (Utilities|Array|Get(acopy) _outactors_6))))
            (:then_2
              (bind _outactors_7 (Actor|GetAllActorsOfClass "/Game/Final_Project_Content/Blueprints/Third_Stage/Second_Boss_Stage/BP_2nd_Boss_Guard3.BP_2nd_Boss_Guard3_C"))
              (bind _asbp_2nd_boss_guard_3 (Utilities|Casting|CastToBP_2nd_Boss_Guard3 (Utilities|Array|Get(acopy) _outactors_7))))
            (:then_3
              (bind _outactors_8 (Actor|GetAllActorsOfClass "/Game/Final_Project_Content/Blueprints/Third_Stage/Second_Boss_Stage/BP_2nd_Boss_Guard4.BP_2nd_Boss_Guard4_C"))
              (bind _asbp_2nd_boss_guard_4 (Utilities|Casting|CastToBP_2nd_Boss_Guard4 (Utilities|Array|Get(acopy) _outactors_8))))))
        (:then_6
          ;[1 1 1] Third Stage is Activated
          (if (and (<= (Variables|Default|GetThird_Boss_Health) 4e+01) (> (Variables|Default|GetThird_Boss_Health) 2e+01))
            (Utilities|FlowControl|DoOnce false
              (:Completed
                (CallFunction|ThirdBossStage)))))
        (:then_7
          ;[1 1 1] boss will reappear after 3rd stage
          (Utilities|FlowControl|Sequence
            (:then_0
              (bind _outactors_9 (Actor|GetAllActorsOfClass "/Game/Final_Project_Content/Blueprints/Third_Stage/Third_Boss_Stage/BP_3rd_Boss_Guard1.BP_3rd_Boss_Guard1_C"))
              (bind _asbp_3rd_boss_guard_1 (Utilities|Casting|CastToBP_3rd_Boss_Guard1 (Utilities|Array|Get(acopy) _outactors_9)))
              (if (Math|Boolean|ANDBoolean (Variables|/Game/Final_Project_Content/Blueprints/Third_Stage/Third_Boss_Stage/BP_3rd_Boss_Guard1.BP_3rd_Boss_Guard1_C|GetDead _asbp_3rd_boss_guard_1) (Variables|/Game/Final_Project_Content/Blueprints/Third_Stage/Third_Boss_Stage/BP_3rd_Boss_Guard2.BP_3rd_Boss_Guard2_C|GetDead (stale _asbp_3rd_boss_guard_2)) (Variables|/Game/Final_Project_Content/Blueprints/Third_Stage/Third_Boss_Stage/BP_3rd_Boss_Guard3.BP_3rd_Boss_Guard3_C|GetDead (stale _asbp_3rd_boss_guard_3)) (Variables|/Game/Final_Project_Content/Blueprints/Third_Stage/Third_Boss_Stage/BP_3rd_Boss_Guard4.BP_3rd_Boss_Guard4_C|GetDead (stale _asbp_3rd_boss_guard_4)))
                (Utilities|FlowControl|DoOnce false
                  (:Completed
                    (Transformation|SetActorLocation "1020.000000, 0,632.000000" false false)))))
            (:then_1
              (bind _outactors_10 (Actor|GetAllActorsOfClass "/Game/Final_Project_Content/Blueprints/Third_Stage/Third_Boss_Stage/BP_3rd_Boss_Guard2.BP_3rd_Boss_Guard2_C"))
              (bind _asbp_3rd_boss_guard_2 (Utilities|Casting|CastToBP_3rd_Boss_Guard2 (Utilities|Array|Get(acopy) _outactors_10))))
            (:then_2
              (bind _outactors_11 (Actor|GetAllActorsOfClass "/Game/Final_Project_Content/Blueprints/Third_Stage/Third_Boss_Stage/BP_3rd_Boss_Guard3.BP_3rd_Boss_Guard3_C"))
              (bind _asbp_3rd_boss_guard_3 (Utilities|Casting|CastToBP_3rd_Boss_Guard3 (Utilities|Array|Get(acopy) _outactors_11))))
            (:then_3
              (bind _outactors_12 (Actor|GetAllActorsOfClass "/Game/Final_Project_Content/Blueprints/Third_Stage/Third_Boss_Stage/BP_3rd_Boss_Guard4.BP_3rd_Boss_Guard4_C"))
              (bind _asbp_3rd_boss_guard_4 (Utilities|Casting|CastToBP_3rd_Boss_Guard4 (Utilities|Array|Get(acopy) _outactors_12))))))
        (:then_8
          ;[1 1 1] Comment
          (if (< (Variables|Default|GetThird_Boss_Health) 2e+01)
            (Utilities|FlowControl|DoOnce false
              (:Completed
                (CallFunction|LastBossStage)))))
        (:then_9
          ;[1 1 1] Comment
          (Utilities|FlowControl|Sequence
            (:then_0
              (bind _outactors_13 (Actor|GetAllActorsOfClass "/Game/Final_Project_Content/Blueprints/Third_Stage/Fourth_Boss_Stage/BP_4th_Boss_Guard.BP_4th_Boss_Guard_C"))
              (bind _asbp_4th_boss_guard (Utilities|Casting|CastToBP_4th_Boss_Guard (Utilities|Array|Get(acopy) _outactors_13)))
              (if (Math|Boolean|ANDBoolean (Variables|/Game/Final_Project_Content/Blueprints/Third_Stage/Fourth_Boss_Stage/BP_4th_Boss_Guard.BP_4th_Boss_Guard_C|GetDead _asbp_4th_boss_guard) (Variables|/Game/Final_Project_Content/Blueprints/Third_Stage/Fourth_Boss_Stage/BP_4th_Boss_Guard2.BP_4th_Boss_Guard2_C|GetDead (stale _asbp_4th_boss_guard_2)) (Variables|/Game/Final_Project_Content/Blueprints/Third_Stage/Fourth_Boss_Stage/BP_4th_Boss_Guard3.BP_4th_Boss_Guard3_C|GetDead (stale _asbp_4th_boss_guard_3)) (Variables|/Game/Final_Project_Content/Blueprints/Third_Stage/Fourth_Boss_Stage/BP_4th_Boss_Guard4.BP_4th_Boss_Guard4_C|GetDead (stale _asbp_4th_boss_guard_4)))
                (Utilities|FlowControl|DoOnce false
                  (:Completed
                    (Transformation|SetActorLocation "1020.000000, 0,632.000000" false false)))))
            (:then_1
              (bind _outactors_14 (Actor|GetAllActorsOfClass "/Game/Final_Project_Content/Blueprints/Third_Stage/Fourth_Boss_Stage/BP_4th_Boss_Guard2.BP_4th_Boss_Guard2_C"))
              (bind _asbp_4th_boss_guard_2 (Utilities|Casting|CastToBP_4th_Boss_Guard2 (Utilities|Array|Get(acopy) _outactors_14))))
            (:then_2
              (bind _outactors_15 (Actor|GetAllActorsOfClass "/Game/Final_Project_Content/Blueprints/Third_Stage/Fourth_Boss_Stage/BP_4th_Boss_Guard3.BP_4th_Boss_Guard3_C"))
              (bind _asbp_4th_boss_guard_3 (Utilities|Casting|CastToBP_4th_Boss_Guard3 (Utilities|Array|Get(acopy) _outactors_15))))
            (:then_3
              (bind _outactors_16 (Actor|GetAllActorsOfClass "/Game/Final_Project_Content/Blueprints/Third_Stage/Fourth_Boss_Stage/BP_4th_Boss_Guard4.BP_4th_Boss_Guard4_C"))
              (bind _asbp_4th_boss_guard_4 (Utilities|Casting|CastToBP_4th_Boss_Guard4 (Utilities|Array|Get(acopy) _outactors_16))))))
        (:then_10
          ;[1 1 1] Comment
          (if (< (Variables|Default|GetThird_Boss_Health) 2e+01)
            (CallFunction|LastAttack)))))))

(event EventBeginPlay
  ;[1 1 1] Health Bar
  (Utilities|FlowControl|Sequence
    (:then_1
      (Class|ActorComponent|SetIsReplicated (Variables|Default|GetPaperFlipbook) true)
      (bind _returnvalue (UserInterface|CreateWidget "/Game/Final_Project_Content/Widgets/Boss_Health.Boss_Health_C"))
      (UserInterface|Viewport|AddtoViewport _returnvalue 0)
      (Variables|Default|SetLocation%20of%20Boss (Transformation|GetActorLocation))
      (Utilities|FlowControl|Delay (Variables|Default|GetStart%20Platform))
      (Variables|Default|SetStart true))))

(fn ConstructionScript)