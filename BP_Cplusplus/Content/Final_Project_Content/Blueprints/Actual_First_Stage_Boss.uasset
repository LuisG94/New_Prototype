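; First-stage boss actor with a Paper2D sprite that faces the player and fires as it moves.
; Each Tick it yaws toward the player character and creeps along +X by a fixed, frame-dependent step.
; When the signed X gap between player controller and sprite falls below a threshold, BOSSAtck spawns BP_Ammo12 at the Arrow, rate-limited by a DoOnce and Delay.
; A mid-range check only re-applies the current location.
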(event OnComponentBeginOverlap(Capsule)
  (params (OverlappedComponent :type Primitive%20Component%20Object%20Reference) (OtherActor :type Actor%20Object%20Reference) (OtherComp :type Primitive%20Component%20Object%20Reference) (OtherBodyIndex :type Integer) (bFromSweep :type Boolean) (SweepResult :type Hit%20Result%20Structure%20%28by%20ref%29)))

(event Custom|BOSSAtck
  ;[1 1 1] Boss_Attack
  (Utilities|FlowControl|DoOnce false :!label _label
    (:Completed
      (Game|SpawnActorfromClass "/Game/Final_Project_Content/Blueprints/Attacks/BP_Ammo12.BP_Ammo12_C" (Transformation|GetWorldTransform (Variables|Default|GetArrow)) "Undefined" 0 0)
      (Utilities|FlowControl|Delay 1.0)
      (goto _label Reset))))

(event EventTick
  (params (DeltaSeconds :type Float%20%28single-precision%29))
  (bind _returnvalue (Transformation|GetActorLocation))
  (bind _returnvalue_2 (Transformation|GetActorLocation))
  (bind (_x _y _z) (Math|Vector|BreakVector _returnvalue))
  (Utilities|FlowControl|Sequence
    (:then_0
      (Transformation|SetActorRotation (Math|Rotator|MakeRotator 0.0 0.0 (.yaw (Math|Rotator|FindLookatRotation (Transformation|GetActorLocation) (Transformation|GetActorLocation (Game|GetPlayerCharacter 0)))))))
    (:then_1
      (bind _output_get (Variables|Default|SetDistance (- (.x (Transformation|GetActorLocation (Game|GetPlayerController 0))) (.x (Transformation|GetWorldLocation (Variables|Default|GetPaperSprite))))))
      (if (<= _output_get 2e+02)
        (CallFunction|BOSSAtck)))
    (:then_2
      (Variables|Default|SetActorX (.x _returnvalue_2)))
    (:then_3
      (Variables|Default|SetActorY (.y _returnvalue_2)))
    (:then_4
      (Variables|Default|SetActorZ (.z _returnvalue_2)))
    (:then_5
      (if (Math|Float|InRange(Float) (Variables|Default|GetDistance) 0.0 4e+02)
        (Transformation|SetActorLocation (Math|Vector|MakeVector (Variables|Default|GetActorX) (Variables|Default|GetActorY) (Variables|Default|GetActorZ)) false false)))
    (:then_6
      (Transformation|SetActorLocation (Math|Vector|MakeVector (+ _x 0.5) _y _z) false false))))

(fn ConstructionScript)