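; Trigger actor that plays the third level's timed text sequence when the 2D side-scroller player character enters its box.
; On overlap it shows two text widgets back to back for a short moment each, plays the SeekandDestroy sound, then after a pause shows a third widget.
; Ending the overlap destroys the actor without checking which actor left, even if the delayed sequence is still running.
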(event OnComponentBeginOverlap(Box)
  (params (OverlappedComponent :type Primitive%20Component%20Object%20Reference) (OtherActor :type Actor%20Object%20Reference) (OtherComp :type Primitive%20Component%20Object%20Reference) (OtherBodyIndex :type Integer) (bFromSweep :type Boolean) (SweepResult :type Hit%20Result%20Structure%20%28by%20ref%29))
  (Utilities|Casting|CastTo2DSideScrollerCharacter0 OtherActor)
  (bind _returnvalue (UserInterface|CreateWidget "/Game/Final_Project_Content/Widgets/Third_lvl_text.Third_lvl_text_C"))
  (UserInterface|Viewport|AddtoViewport _returnvalue 0)
  (Utilities|FlowControl|Delay 1.4)
  (Widget|RemovefromParent _returnvalue)
  (bind _returnvalue_2 (UserInterface|CreateWidget "/Game/Final_Project_Content/Widgets/Third_lvl_text1.Third_lvl_text1_C"))
  (UserInterface|Viewport|AddtoViewport _returnvalue_2 0)
  (Utilities|FlowControl|Delay 1.4)
  (Widget|RemovefromParent _returnvalue_2)
  (Audio|PlaySound2D "/Game/Final_Project_Content/Sound_Music/SeekandDestroy.SeekandDestroy" 1.0 1.0 0.0 0 0)
  (Utilities|FlowControl|Delay 4.0)
  (bind _returnvalue_3 (UserInterface|CreateWidget "/Game/Final_Project_Content/Widgets/Third_lvl_text2.Third_lvl_text2_C"))
  (UserInterface|Viewport|AddtoViewport _returnvalue_3 0)
  (Utilities|FlowControl|Delay 1.4)
  (Widget|RemovefromParent _returnvalue_3))

(event OnComponentEndOverlap(Box)
  (params (OverlappedComponent :type Primitive%20Component%20Object%20Reference) (OtherActor :type Actor%20Object%20Reference) (OtherComp :type Primitive%20Component%20Object%20Reference) (OtherBodyIndex :type Integer))
  (Actor|DestroyActor))

(fn ConstructionScript)