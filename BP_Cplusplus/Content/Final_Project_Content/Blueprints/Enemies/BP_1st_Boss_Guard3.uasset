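; BP_1st_Boss_Guard3 is a first-stage boss guard with attack and damage events.
; The damage event only subtracts incoming damage from health, and the attack event only enters a DoOnce.
; Unconnected chains hold the intended behavior: spawning BP_Boss_Ammo with a delayed DoOnce reset, and an explosion sound plus destruction at zero health.
; As wired, the guard neither fires nor dies.
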(event Custom|First_Stage_Guard
  (params (DMG%20In :type Float%20%28single-precision%29))
  ;[1 1 1] damageboss
  (bind _output_get (Variables|Default|SetFirst_Stage_Guard_Health (- (Variables|Default|GetFirst_Stage_Guard_Health) DMG%20In))))

(event Custom|1st_First_Stage_Guard_Attk
  ;[1 1 1] boss attack
  (Utilities|FlowControl|DoOnce false))

(event EventBeginPlay)

(event Collision|EventActorBeginOverlap
  (params (OtherActor :type Actor%20Object%20Reference)))

(event EventTick
  (params (DeltaSeconds :type Float%20%28single-precision%29)))

(fn ConstructionScript)