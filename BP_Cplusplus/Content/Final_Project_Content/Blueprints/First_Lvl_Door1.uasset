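; First-level door actor that plays its opening flipbook animation when play begins.
; BeginPlay assigns the opening flipbook to the DoorClosingFlipbook component, then stops it after a short delay.
; Disconnected nodes hold an unused closing animation and a check of the First_Transition_Terminal_Text actor's OpenDoor flag to open the door, neither of which runs.
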(event EventBeginPlay
  (bind _door_closing_flipbook (Variables|Default|GetDoor_Closing_Flipbook))
  (Sprite|SetFlipbook _door_closing_flipbook "/Game/Final_Project_Content/Sprites/Textures/Door_Opening_Flipbook.Door_Opening_Flipbook")
  (Utilities|FlowControl|Delay 1.4)
  (Audio|Components|Audio|Stop _door_closing_flipbook))

(fn ConstructionScript)