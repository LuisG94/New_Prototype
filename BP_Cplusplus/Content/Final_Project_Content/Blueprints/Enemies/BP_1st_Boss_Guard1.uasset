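; First-stage boss guard enemy that fires boss ammo and can be destroyed by damage.
; Its attack event spawns BP_Boss_Ammo at the FirstArrow transform, with a DoOnce reset after a delay acting as a fire-rate cooldown.
; Its damage event subtracts from guard health, then plays an explosion sound and destroys the actor when health runs out.
; The First_Box overlap event is empty, and nothing in this graph triggers the attack.
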(event OnComponentBeginOverlap(First_Box)
  (params (OverlappedComponent :type Primitive%20Component%20Object%20Reference) (OtherActor :type Actor%20Object%20Reference) (OtherComp :type Primitive%20Component%20Object%20Reference) (OtherBodyIndex :type Integer) (bFromSweep :type Boolean) (SweepResult :type Hit%20Result%20Structure%20%28by%20ref%29)))

(event Custom|damage
  (params (DMG%20In :type Float%20%28single-precision%29))
  ;[1 1 1] damage guard
  (bind _output_get (Variables|Default|SetFirst_Stage_Guard_Health (- (Variables|Default|GetFirst_Stage_Guard_Health) DMG%20In)))
  (if (<= _output_get 0.0)
    (Audio|PlaySound2D "/Game/Final_Project_Content/Sound_Music/SoundsCrate-SciFi-Explosion5__1_.SoundsCrate-SciFi-Explosion5__1_" 1.0 1.0 0.0 0 0)
    (Actor|DestroyActor)))

(event Custom|1st_First_Stage_Guard_Attk
  ;[1 1 1] Guard attk
  (Utilities|FlowControl|DoOnce false :!label _label
    (:Completed
      (Game|SpawnActorfromClass "/Game/Final_Project_Content/Blueprints/Attacks/BP_Boss_Ammo.BP_Boss_Ammo_C" (Transformation|GetWorldTransform (Variables|Default|GetFirst_Arrow)) "Undefined" 0 0)
      (Utilities|FlowControl|Delay 1.5)
      (goto _label Reset))))

(event EventBeginPlay)

(event Collision|EventActorBeginOverlap
  (params (OtherActor :type Actor%20Object%20Reference)))

(event EventTick
  (params (DeltaSeconds :type Float%20%28single-precision%29)))

(fn ConstructionScript)