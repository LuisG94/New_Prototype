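; BP_Turret is a 2D sprite enemy turret that fires BP_Ammo1 from its Arrow component when the player is near.
; Tick measures the signed X offset to the player and triggers shooting at 400 or less, throttled by a DoOnce that resets after a two-second delay.
; Its damage event derives health from DistanceToPlayer minus damage rather than from stored health, destroying the turret with a sound at zero or below.
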(event Custom|Turret_Shooting
  ;[1 1 1] Turret_Shooting
  (Utilities|FlowControl|DoOnce false :!label _label
    (:Completed
      (Game|SpawnActorfromClass "/Game/Final_Project_Content/Blueprints/Attacks/BP_Ammo1.BP_Ammo1_C" (Transformation|GetWorldTransform (Variables|Default|GetArrow)) "Undefined" 0 0)
      (Utilities|FlowControl|Delay 2.0)
      (goto _label Reset))))

(event Custom|TurretHealth
  (params (DamageReceived :type Float%20%28single-precision%29))
  ;[1 1 1] Turret Health System
  (bind _output_get (Variables|Default|SetTurret_Health (- (Variables|Default|GetDistance_To_Player) DamageReceived)))
  (if (<= _output_get 0.0)
    (Actor|DestroyActor)
    (Audio|PlaySound2D 0 1.0 1.0 0.0 0 0)))

(event EventTick
  (params (DeltaSeconds :type Float%20%28single-precision%29))
  ;[1 1 1] If player is within certain distance attack player
  (Utilities|FlowControl|Sequence
    (:then_0
      (bind _output_get (Variables|Default|SetDistance_To_Player (- (.x (Transformation|GetWorldLocation (Variables|Default|GetPaperSprite))) (.x (Transformation|GetActorLocation (Game|GetPlayerCharacter 0))))))
      (if (<= _output_get 4e+02)
        (CallFunction|TurretShooting)))))

(fn ConstructionScript)