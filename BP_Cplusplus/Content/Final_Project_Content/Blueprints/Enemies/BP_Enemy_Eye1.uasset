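; BP_Enemy_Eye1 is a Paper2D eye enemy that shoots when the player is near on the X axis.
; Tick compares signed X distance to the player against a threshold, firing BP_Enemy_Eye_Ammo1 from an Arrow, throttled by a DoOnce reset after a Delay.
; When Start is set, a Timeline moves it as an offset from LocationofPlat1.
; DMG_Enemy subtracts health, destroying the actor with a balloon-burst sound at zero.
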(event Custom|DMG_Enemy
  (params (Dmg%20In :type Float%20%28single-precision%29))
  ;[1 1 1] Damage Received
  (bind _output_get (Variables|Default|SetEnemy_Health (- (Variables|Default|GetEnemy_Health) Dmg%20In)))
  (if (<= _output_get 0.0)
    (Actor|DestroyActor)
    (Audio|PlaySound2D "/Game/Final_Project_Content/Sound_Music/82109__gniffelbaf__balloon-burst-01.82109__gniffelbaf__balloon-burst-01" 1.0 1.0 0.0 0 0)))

(event Custom|Enemy_Attk
  ;[1 1 1] Shooting
  (Utilities|FlowControl|DoOnce false :!label _label
    (:Completed
      (Game|SpawnActorfromClass "/Game/Final_Project_Content/Blueprints/Attacks/BP_Enemy_Eye_Ammo1.BP_Enemy_Eye_Ammo1_C" (Transformation|GetWorldTransform (Variables|Default|GetArrow)) "Undefined" 0 0)
      (Utilities|FlowControl|Delay 2.0)
      (goto _label Reset))))

(event EventBeginPlay)

(event Collision|EventActorBeginOverlap
  (params (OtherActor :type Actor%20Object%20Reference)))

(event EventTick
  (params (DeltaSeconds :type Float%20%28single-precision%29))
  ;[1 1 1] If player is within certain distance attack player
  (Utilities|FlowControl|Sequence
    (:then_0
      (bind _output_get (Variables|Default|SetDistance (- (.x (Transformation|GetWorldLocation (Variables|Default|GetPaperSprite))) (.x (Transformation|GetActorLocation (Game|GetPlayerCharacter 0))))))
      (if (<= _output_get 4e+02)
        (CallFunction|EnemyAttk)))
    (:then_1
      (if (Variables|Default|GetStart)
        (bind _newtrack_0 (Timeline|Timeline_0 Play)
          (:Update
            (Transformation|SetActorLocation (+ (Variables|Default|GetLocationofPlat1) _newtrack_0) false false)))))))

(fn ConstructionScript)