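; Second-stage boss, a Paper2D sprite actor that chases the player along X and shoots at them.
; Each Tick it yaws toward the player, always creeps along +X with extra speed when far behind, and steps vertically to hover above the player.
; Within the X-distance threshold it spawns BP_Boss_Ammo from its Arrow, throttled by a DoOnce and Delay.
; Movement uses fixed per-frame offsets without delta time or sweep.
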(event Custom|Second_Boss_Atck
  ;[1 1 1] Boss_Attack
  (Utilities|FlowControl|DoOnce false :!label _label
    (:Completed
      (Game|SpawnActorfromClass "/Game/Final_Project_Content/Blueprints/Attacks/BP_Boss_Ammo.BP_Boss_Ammo_C" (Transformation|GetWorldTransform (Variables|Default|GetArrow)) "Undefined" 0 0)
      (Utilities|FlowControl|Delay 1.0)
      (goto _label Reset))))

(event EventTick
  (params (DeltaSeconds :type Float%20%28single-precision%29))
  (bind _returnvalue (Transformation|GetActorLocation))
  (bind _returnvalue_2 (Transformation|GetActorLocation))
  (bind _returnvalue_3 (Transformation|GetActorLocation))
  (bind _returnvalue_4 (Transformation|GetActorLocation))
  (bind _returnvalue_5 (Transformation|GetActorLocation))
  (bind (_x _y _z) (Math|Vector|BreakVector _returnvalue_3))
  (bind (_x_2 _y_2 _z_2) (Math|Vector|BreakVector _returnvalue))
  (bind (_x_3 _y_3 _z_3) (Math|Vector|BreakVector _returnvalue_4))
  (bind (_x_4 _y_4 _z_4) (Math|Vector|BreakVector _returnvalue_5))
  (Utilities|FlowControl|Sequence
    (:then_0
      (Transformation|SetActorRotation (Math|Rotator|MakeRotator 0.0 0.0 (.yaw (Math|Rotator|FindLookatRotation (Transformation|GetActorLocation) (Transformation|GetActorLocation (Game|GetPlayerCharacter 0)))))))
    (:then_1
      (bind _output_get (Variables|Default|SetSecond_Boss_X_Distance (- (.x (Transformation|GetActorLocation (Game|GetPlayerCharacter 0))) (.x (Transformation|GetWorldLocation (Variables|Default|GetPaperSprite))))))
      (if (<= _output_get 3e+02)
        (CallFunction|SecondBossAtck)))
    (:then_2
      (Variables|Default|SetActorX (.x _returnvalue_2)))
    (:then_3
      (Variables|Default|SetActorY (.y _returnvalue_2)))
    (:then_4
      (Variables|Default|SetActorZ (.z _returnvalue_2)))
    (:then_5
      (if (Math|Float|InRange(Float) (Variables|Default|GetSecond_Boss_X_Distance) 0.0 4e+02)
        (Transformation|SetActorLocation (Math|Vector|MakeVector (Variables|Default|GetActorX) (Variables|Default|GetActorY) (Variables|Default|GetActorZ)) false false)))
    (:then_7
      (bind _output_get_2 (Variables|Default|SetSecond_Boss_X_Distance (- (.x (Transformation|GetActorLocation (Game|GetPlayerCharacter 0))) (.x (Transformation|GetWorldLocation (Variables|Default|GetPaperSprite))))))
      (if (>= _output_get_2 3e+02)
        (Transformation|SetActorLocation (Math|Vector|MakeVector (+ _x_3 1.6) _y_3 _z_3) false false)))
    (:then_8
      (Transformation|SetActorLocation (Math|Vector|MakeVector (+ _x 1.2) _y _z) false false))
    (:then_9
      (bind _output_get_3 (Variables|Default|SetSecond_Boss_Z_Distance (- (.z (Transformation|GetActorLocation (Game|GetPlayerCharacter 0))) (.z (Transformation|GetWorldLocation (Variables|Default|GetPaperSprite))))))
      (if (> _output_get_3 -7e+01)
        (Transformation|SetActorLocation (Math|Vector|MakeVector _x_4 _y_4 (+ _z_4 0.75)) false false)
        (else
          (Transformation|SetActorLocation (Math|Vector|MakeVector _x_2 _y_2 (- _z_2 0.75)) false false))))))

(fn ConstructionScript)