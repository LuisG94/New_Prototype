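; BP_Enemy_Eye2 is a Paper2D enemy that moves along a timeline path and fires at the player.
; After a StartPlat delay, Tick plays the timeline, offsetting the actor from its starting location.
; Tick triggers attacks when sprite X minus player X is at most 400, a signed check; a DoOnce spawns BP_Boss_Ammo at the Arrow with a two-second cooldown.
; DMG_Enemy reduces health, destroying the actor with a pop sound at zero.
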(event Custom|DMG_Enemy
  (params (Dmg%20In :type Float%20%28single-precision%29))
  ;[1 1 1] Damage Received
  (bind _output_get (Variables|Default|SetEnemy_Health (- (Variables|Default|GetEnemy_Health) Dmg%20In)))
  (if (<= _output_get 0.0)
    (Actor|DestroyActor)
    (Audio|PlaySound2D "/Game/Final_Project_Content/Sound_Music/82109__gniffelbaf__balloon-burst-01.82109__gniffelbaf__balloon-burst-01" 1.0 1.0 0.0 0 0)))

(event Custom|Enemy_Attk
  ;[1 1 1] Shooting
  (Utilities|FlowControl|DoOnce false :!label _label
    (:Completed
      (Game|SpawnActorfromClass "/Game/Final_Project_Content/Blueprints/Attacks/BP_Boss_Ammo.BP_Boss_Ammo_C" (Transformation|GetWorldTransform (Variables|Default|GetArrow)) "Undefined" 0 0)
      (Utilities|FlowControl|Delay 2.0)
      (goto _label Reset))))

(event Collision|EventActorBeginOverlap
  (params (OtherActor :type Actor%20Object%20Reference)))

(event EventBeginPlay
  ;[1 1 1] Start trigger for platform
  (Variables|Default|SetLocationofPlat (Transformation|GetActorLocation))
  (Utilities|FlowControl|Delay (Variables|Default|GetStartPlat))
  (Variables|Default|SetStart true))

(event EventTick
  (params (DeltaSeconds :type Float%20%28single-precision%29))
  ;[1 1 1] If player is within certain distance attack player
  (Utilities|FlowControl|Sequence
    (:then_0
      (bind _output_get (Variables|Default|SetDistance (- (.x (Transformation|GetWorldLocation (Variables|Default|GetPaperSprite))) (.x (Transformation|GetActorLocation (Game|GetPlayerCharacter 0))))))
      (if (<= _output_get 4e+02)
        (CallFunction|EnemyAttk)))
    (:then_1
      (if (Variables|Default|GetStart)
        (Utilities|FlowControl|Sequence
          (:then_0
            (bind _newtrack_0 (Timeline|Timeline_0 Play)
              (:Update
                (Transformation|SetActorLocation (+ _newtrack_0 (Variables|Default|GetLocationofPlat)) false false)))))))))

(fn ConstructionScript)