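; BP_1st_Boss_Guard2 is a destructible guard for the first boss stage.
; Its damage event subtracts from health and, at zero or below, sets Dead, destroys the arrow, box and paper sprite components, and plays an explosion sound.
; The attack event only enters a DoOnce, leaving the boss ammo spawn and delayed reset unconnected, so it never fires.
; The actor itself is not destroyed on death.
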(event Custom|damage
  (params (DMG%20In :type Float%20%28single-precision%29))
  ;[1 1 1] damageboss
  (bind _output_get (Variables|Default|SetFirst_Stage_Guard_Health (- (Variables|Default|GetFirst_Stage_Guard_Health) DMG%20In)))
  (if (<= _output_get 0.0)
    (Variables|Default|SetDead true)
    (Utilities|FlowControl|Sequence
      (:then_0
        (Components|DestroyComponent (Variables|Default|GetFirst_Arrow)))
      (:then_1
        (Components|DestroyComponent (Variables|Default|GetFirst_Box)))
      (:then_2
        (Components|DestroyComponent (Variables|Default|GetFirst_PaperSprite)))
      (:then_3
        (Audio|PlaySound2D "/Game/Final_Project_Content/Sound_Music/SoundsCrate-SciFi-Explosion5__1_.SoundsCrate-SciFi-Explosion5__1_" 1.0 1.0 0.0 0 0)))))

(event Custom|2nd_First_Stage_Guard_Attk
  ;[1 1 1] boss attack
  (Utilities|FlowControl|DoOnce false))

(event EventBeginPlay)

(event Collision|EventActorBeginOverlap
  (params (OtherActor :type Actor%20Object%20Reference)))

(event EventTick
  (params (DeltaSeconds :type Float%20%28single-precision%29)))

(fn ConstructionScript)