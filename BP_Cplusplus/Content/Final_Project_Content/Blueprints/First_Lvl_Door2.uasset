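; First_Lvl_Door2 is a Paper2D flipbook door that plays its opening animation once the Third_Stage_Boss is dead.
; Every Tick it finds the first boss actor by class and polls its Dead flag.
; When the flag is set, it swaps to the opening flipbook and stops playback after a short Delay.
; Disconnected nodes hold unused closing logic and an older terminal-triggered opening with a debug print.
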(event EventTick
  (params (DeltaSeconds :type Float%20%28single-precision%29))
  (bind _door_closing_flipbook (Variables|Default|GetDoor_Closing_Flipbook))
  (bind _outactors (Actor|GetAllActorsOfClass "/Game/Final_Project_Content/Blueprints/Third_Stage/Third_Stage_Boss.Third_Stage_Boss_C"))
  (bind _asthird_stage_boss (Utilities|Casting|CastToThird_Stage_Boss (Utilities|Array|Get(acopy) _outactors)))
  (if (Variables|/Game/Final_Project_Content/Blueprints/Third_Stage/Third_Stage_Boss.Third_Stage_Boss_C|GetDead _asthird_stage_boss)
    (Sprite|SetFlipbook _door_closing_flipbook "/Game/Final_Project_Content/Sprites/Textures/Door_Opening_Flipbook.Door_Opening_Flipbook")
    (Utilities|FlowControl|Delay 1.2)
    (Audio|Components|Audio|Stop _door_closing_flipbook)))

(fn ConstructionScript)