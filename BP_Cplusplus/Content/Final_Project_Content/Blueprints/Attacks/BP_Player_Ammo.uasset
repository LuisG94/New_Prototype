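; BP_Player_Ammo is the player's ammo actor, which damages enemies and the boss on overlap.
; It has four capsule components, each with an overlap event that casts to one target class: three Enemy Eye variants and Boss1.
; A matching hit calls that target's damage function with a fixed per-type amount and destroys the ammo.
; Other overlaps are ignored, and this graph contains no movement logic.
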(event OnComponentBeginOverlap(Capsule1)
  (params (OverlappedComponent :type Primitive%20Component%20Object%20Reference) (OtherActor :type Actor%20Object%20Reference) (OtherComp :type Primitive%20Component%20Object%20Reference) (OtherBodyIndex :type Integer) (bFromSweep :type Boolean) (SweepResult :type Hit%20Result%20Structure%20%28by%20ref%29))
  (bind _asbp_enemy_eye (Utilities|Casting|CastToBP_Enemy_Eye OtherActor))
  (Default|DMGEnemy _asbp_enemy_eye 5e+01)
  (Actor|DestroyActor))

(event OnComponentBeginOverlap(Capsule)
  (params (OverlappedComponent :type Primitive%20Component%20Object%20Reference) (OtherActor :type Actor%20Object%20Reference) (OtherComp :type Primitive%20Component%20Object%20Reference) (OtherBodyIndex :type Integer) (bFromSweep :type Boolean) (SweepResult :type Hit%20Result%20Structure%20%28by%20ref%29))
  (bind _asbp_enemy_eye_1 (Utilities|Casting|CastToBP_Enemy_Eye1 OtherActor))
  (Default|DMGEnemy _asbp_enemy_eye_1 5.0)
  (Actor|DestroyActor))

(event OnComponentBeginOverlap(Capsule2)
  (params (OverlappedComponent :type Primitive%20Component%20Object%20Reference) (OtherActor :type Actor%20Object%20Reference) (OtherComp :type Primitive%20Component%20Object%20Reference) (OtherBodyIndex :type Integer) (bFromSweep :type Boolean) (SweepResult :type Hit%20Result%20Structure%20%28by%20ref%29))
  (bind _asbp_enemy_eye_2 (Utilities|Casting|CastToBP_Enemy_Eye2 OtherActor))
  (Default|DMGEnemy _asbp_enemy_eye_2 5.0)
  (Actor|DestroyActor))

(event OnComponentBeginOverlap(Capsule3)
  (params (OverlappedComponent :type Primitive%20Component%20Object%20Reference) (OtherActor :type Actor%20Object%20Reference) (OtherComp :type Primitive%20Component%20Object%20Reference) (OtherBodyIndex :type Integer) (bFromSweep :type Boolean) (SweepResult :type Hit%20Result%20Structure%20%28by%20ref%29))
  (bind _asboss_1 (Utilities|Casting|CastToBoss1 OtherActor))
  (Default|DMGBOSS _asboss_1 1e+01)
  (Actor|DestroyActor))

(event EventBeginPlay)

(event Collision|EventActorBeginOverlap
  (params (OtherActor :type Actor%20Object%20Reference)))

(event EventTick
  (params (DeltaSeconds :type Float%20%28single-precision%29)))

(fn ConstructionScript)