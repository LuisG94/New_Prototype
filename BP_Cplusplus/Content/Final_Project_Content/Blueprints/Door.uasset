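; Door actor, apparently 2D, that displays its motion through a Paper2D flipbook component.
; On BeginPlay it assigns the opening flipbook and immediately stops playback, so the door holds still.
; Unconnected leftover nodes would play a closing animation, or check the OpenDoor flag on First_Transition_Terminal_Text and play the opening animation briefly.
; None of that leftover logic runs, so this graph never animates the door.
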(event EventBeginPlay
  (bind _door_closing_flipbook (Variables|Default|GetDoor_Closing_Flipbook))
  (Sprite|SetFlipbook _door_closing_flipbook "/Game/Final_Project_Content/Sprites/Textures/Door_Opening_Flipbook.Door_Opening_Flipbook")
  (Audio|Components|Audio|Stop _door_closing_flipbook))

(fn ConstructionScript)