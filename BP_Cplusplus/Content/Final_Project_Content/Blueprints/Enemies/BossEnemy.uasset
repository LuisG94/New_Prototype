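; BossEnemy is a boss actor that shoots at the player and is destroyed when its health runs out.
; Tick yaws it toward the player character and triggers attacks when the signed X offset from the player controller's location is at most 100.
; Attacks spawn BP_Ammo1 at the Arrow, throttled by a DoOnce reset after a delay.
; Any Sphere overlap applies fixed damage, without checking what hit it.
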(event OnComponentBeginOverlap(Sphere)
  (params (OverlappedComponent :type Primitive%20Component%20Object%20Reference) (OtherActor :type Actor%20Object%20Reference) (OtherComp :type Primitive%20Component%20Object%20Reference) (OtherBodyIndex :type Integer) (bFromSweep :type Boolean) (SweepResult :type Hit%20Result%20Structure%20%28by%20ref%29))
  ;[1 1 1] damageboss
  (CallFunction|DMGBoss 25.0))

(event Custom|DMG%20Boss
  (params (DMG%20In :type Float%20%28single-precision%29))
  ;[1 1 1] damageboss
  (bind _output_get (Variables|Default|SetBossHealth (- (Variables|Default|GetBossHealth) DMG%20In)))
  (if (<= _output_get 0.0)
    (Actor|DestroyActor)))

(event Custom|BossAtck
  (Utilities|FlowControl|DoOnce false :!label _label
    (:Completed
      (Game|SpawnActorfromClass "/Game/Final_Project_Content/Blueprints/Attacks/BP_Ammo1.BP_Ammo1_C" (Transformation|GetWorldTransform (Variables|Default|GetArrow)) "Undefined" 0 0)
      (Utilities|FlowControl|Delay 0.6)
      (goto _label Reset))))

(event EventBeginPlay)

(event Collision|EventActorBeginOverlap
  (params (OtherActor :type Actor%20Object%20Reference)))

(event EventTick
  (params (DeltaSeconds :type Float%20%28single-precision%29))
  (Utilities|FlowControl|Sequence
    (:then_0
      (bind _output_get (Variables|Default|SetDistance (- (.x (Transformation|GetWorldLocation (Variables|Default|GetPaperSprite))) (.x (Transformation|GetActorLocation (Game|GetPlayerController 0))))))
      (if (<= _output_get 1e+02)
        (CallFunction|BossAtck)))
    (:then_1
      (Transformation|SetActorRotation (Math|Rotator|MakeRotator 0.0 0.0 (.yaw (Math|Rotator|FindLookatRotation (Transformation|GetActorLocation) (Transformation|GetActorLocation (Game|GetPlayerCharacter 0)))))))))

(fn ConstructionScript)