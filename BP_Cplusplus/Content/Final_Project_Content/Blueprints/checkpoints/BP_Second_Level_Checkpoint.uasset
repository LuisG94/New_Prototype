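; Second-level checkpoint trigger that saves the player ship's location when a "Ship"-tagged actor overlaps it.
; Each overlap creates a BP_Second_Level_Save_Info object, and a DoOnce writes the Space_Ship11 location into it and saves to slot "Loc" only once.
; The construction script sizes the box from a variable and uses SecondStageCheckpoint to pick a Checkpoint or Save billboard sprite.
; That flag also branches the save logic, but both paths are identical.
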(event EventBeginPlay)

(event Collision|EventActorBeginOverlap
  (params (OtherActor :type Actor%20Object%20Reference))
  (if (Actor|ActorHasTag OtherActor "Ship")
    (bind _returnvalue (SaveGame|CreateSaveGameObject "/Game/Final_Project_Content/Blueprints/checkpoints/BP_Second_Level_Save_Info.BP_Second_Level_Save_Info_C"))
    (bind _asbp_second_level_save_info (Utilities|Casting|CastToBP_Second_Level_Save_Info _returnvalue))
    (Variables|Default|SetSecond_Stage_Save_Info _asbp_second_level_save_info)
    (bind _asspace_ship_11 (Utilities|Casting|CastToSpace_Ship11 (Game|GetPlayerCharacter 0)))
    (Variables|Default|SetShip%20Info _asspace_ship_11)
    (if (Variables|Default|GetSecondStageCheckpoint)
      (Utilities|FlowControl|DoOnce false
        (:Completed
          (Variables|/Game/Final_Project_Content/Blueprints/checkpoints/BP_Second_Level_Save_Info.BP_Second_Level_Save_Info_C|SetSecondStageCheckLocation (Variables|Default|GetSecond_Stage_Save_Info) (Math|Vector|MakeVector (.x (Transformation|GetActorLocation (Variables|Default|GetShip%20Info))) (.y (Transformation|GetActorLocation (Variables|Default|GetShip%20Info))) (.z (Transformation|GetActorLocation (Variables|Default|GetShip%20Info)))))
          (SaveGame|SaveGametoSlot (Variables|Default|GetSecond_Stage_Save_Info) "Loc")))
      (else
        (Utilities|FlowControl|DoOnce false
          (:Completed
            (Variables|/Game/Final_Project_Content/Blueprints/checkpoints/BP_Second_Level_Save_Info.BP_Second_Level_Save_Info_C|SetSecondStageCheckLocation (Variables|Default|GetSecond_Stage_Save_Info) (Math|Vector|MakeVector (.x (Transformation|GetActorLocation (Variables|Default|GetShip%20Info))) (.y (Transformation|GetActorLocation (Variables|Default|GetShip%20Info))) (.z (Transformation|GetActorLocation (Variables|Default|GetShip%20Info)))))
            (SaveGame|SaveGametoSlot (Variables|Default|GetSecond_Stage_Save_Info) "Loc")))))))

(event EventTick
  (params (DeltaSeconds :type Float%20%28single-precision%29)))

(fn ConstructionScript
  (Components|Box|SetBoxExtent (Variables|Default|GetBox) (Variables|Default|GetChange%20Second%20Stage%20Hit%20Box) true)
  (if (Variables|Default|GetSecondStageCheckpoint)
    (Rendering|Components|Sprite|SetSprite (Variables|Default|GetBillboard) "/Game/Final_Project_Content/Blueprints/checkpoints/checkpoint.checkpoint")
    (else
      (Rendering|Components|Sprite|SetSprite (Variables|Default|GetBillboard) "/Game/Final_Project_Content/Blueprints/checkpoints/save.save"))))