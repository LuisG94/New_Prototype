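; BP_Human_Enemy is a human enemy Blueprint that takes damage and is destroyed when its health runs out.
; DMG_Human_Enemy subtracts incoming damage from HumanEnemyHealth and destroys the actor at zero or below.
; The shooting attack event Human_Enemy_Attk is empty.
; Leftover unconnected nodes for a balloon-burst sound and a DoOnce-gated spawn at the Arrow transform with a delayed reset never run.
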(event Custom|DMG_Human_Enemy
  (params (Dmg%20In :type Float%20%28single-precision%29))
  ;[1 1 1] Damage system for human enemy
  (bind _output_get (Variables|Default|SetHuman_Enemy_Health (- (Variables|Default|GetHuman_Enemy_Health) Dmg%20In)))
  (if (<= _output_get 0.0)
    (Actor|DestroyActor)))

(event Custom|Human_Enemy_Attk
  ;[1 1 1] Shooting attack for human enemy
)

(event EventBeginPlay)

(event Collision|EventActorBeginOverlap
  (params (OtherActor :type Actor%20Object%20Reference)))

(event EventTick
  (params (DeltaSeconds :type Float%20%28single-precision%29)))

(fn ConstructionScript)