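; First-level checkpoint trigger that saves the player character's location when an actor tagged "Tommy" overlaps it.
; Each overlap creates a fresh save-info object, but DoOnce limits writing to the "Location" slot to the first pass, then a debug print shows the stored location.
; The Checkpoint flag picks the billboard sprite in construction, which also sizes the hit box; both flag branches save identically.
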(event EventBeginPlay)

(event EventTick
  (params (DeltaSeconds :type Float%20%28single-precision%29)))

(event Collision|EventActorBeginOverlap
  (params (OtherActor :type Actor%20Object%20Reference))
  (if (Actor|ActorHasTag OtherActor "Tommy")
    (bind _returnvalue (SaveGame|CreateSaveGameObject "/Game/Final_Project_Content/checkpoints/BP_First_Level_Save_info.BP_First_Level_Save_info_C"))
    (bind _asbp_first_level_save_info (Utilities|Casting|CastToBP_First_Level_Save_info _returnvalue))
    (Variables|Default|SetSaveInfo _asbp_first_level_save_info)
    (bind _as2dside_scroller_character_0 (Utilities|Casting|CastTo2DSideScrollerCharacter0 (Game|GetPlayerCharacter 0)))
    (Variables|Default|SetCharInfo _as2dside_scroller_character_0)
    (if (Variables|Default|GetCheckpoint)
      (Utilities|FlowControl|DoOnce false
        (:Completed
          (Variables|/Game/Final_Project_Content/checkpoints/BP_First_Level_Save_info.BP_First_Level_Save_info_C|SetCheckLocation (Variables|Default|GetSaveInfo) (Math|Vector|MakeVector (.x (Transformation|GetActorLocation (Variables|Default|GetCharInfo))) (.y (Transformation|GetActorLocation (Variables|Default|GetCharInfo))) (.z (Transformation|GetActorLocation (Variables|Default|GetCharInfo)))))
          (SaveGame|SaveGametoSlot (Variables|Default|GetSaveInfo) "Location")))
      (else
        (Utilities|FlowControl|DoOnce false
          (:Completed
            (Variables|/Game/Final_Project_Content/checkpoints/BP_First_Level_Save_info.BP_First_Level_Save_info_C|SetCheckLocation (Variables|Default|GetSaveInfo) (Math|Vector|MakeVector (.x (Transformation|GetActorLocation (Variables|Default|GetCharInfo))) (.y (Transformation|GetActorLocation (Variables|Default|GetCharInfo))) (.z (Transformation|GetActorLocation (Variables|Default|GetCharInfo)))))
            (SaveGame|SaveGametoSlot (Variables|Default|GetSaveInfo) "Location")))))
    (Development|PrintString (Utilities|String|ToString(Vector) (Variables|/Game/Final_Project_Content/checkpoints/BP_First_Level_Save_info.BP_First_Level_Save_info_C|GetCheckLocation (Variables|Default|GetSaveInfo))))))

(fn ConstructionScript
  (Components|Box|SetBoxExtent (Variables|Default|GetBox) (Variables|Default|GetChange%20Hit%20Box) true)
  (if (Variables|Default|GetCheckpoint)
    (Rendering|Components|Sprite|SetSprite (Variables|Default|GetBillboard) "/Game/Final_Project_Content/checkpoints/checkpoint.checkpoint")
    (else
      (Rendering|Components|Sprite|SetSprite (Variables|Default|GetBillboard) "/Game/Final_Project_Content/checkpoints/save.save"))))