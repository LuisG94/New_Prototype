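; Trigger actor for a terminal text sequence in the first transition, started when a Transition_Character overlaps its Box.
; It disables the character's input and shows three text widgets in turn for three seconds each, timed with chained Delays.
; It sets the Alarm flag before the last message, then sets OpenDoor and restores input once the sequence ends.
; Nothing here reads either flag or guards against retriggering.
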(event OnComponentBeginOverlap(Box)
  (params (OverlappedComponent :type Primitive%20Component%20Object%20Reference) (OtherActor :type Actor%20Object%20Reference) (OtherComp :type Primitive%20Component%20Object%20Reference) (OtherBodyIndex :type Integer) (bFromSweep :type Boolean) (SweepResult :type Hit%20Result%20Structure%20%28by%20ref%29))
  (bind _astransition_character (Utilities|Casting|CastToTransition_Character OtherActor))
  (Input|DisableInput _astransition_character 0)
  (bind _returnvalue (UserInterface|CreateWidget "/Game/Final_Project_Content/Widgets/First_Transition_text.First_Transition_text_C"))
  (UserInterface|Viewport|AddtoViewport _returnvalue 0)
  (Utilities|FlowControl|Delay 3.0)
  (Widget|RemovefromParent _returnvalue)
  (bind _returnvalue_2 (UserInterface|CreateWidget "/Game/Final_Project_Content/Widgets/First_Transition_text1.First_Transition_text1_C"))
  (UserInterface|Viewport|AddtoViewport _returnvalue_2 0)
  (Utilities|FlowControl|Delay 3.0)
  (Widget|RemovefromParent _returnvalue_2)
  (Variables|Default|SetAlarm true)
  (Utilities|FlowControl|Delay 0.2)
  (bind _returnvalue_3 (UserInterface|CreateWidget "/Game/Final_Project_Content/Widgets/First_Transition_text2.First_Transition_text2_C"))
  (UserInterface|Viewport|AddtoViewport _returnvalue_3 0)
  (Utilities|FlowControl|Delay 3.0)
  (Widget|RemovefromParent _returnvalue_3)
  (Variables|Default|SetOpen_Door true)
  (Input|EnableInput _astransition_character 0))

(event EventBeginPlay)

(event Collision|EventActorBeginOverlap
  (params (OtherActor :type Actor%20Object%20Reference)))

(event EventTick
  (params (DeltaSeconds :type Float%20%28single-precision%29)))

(fn ConstructionScript)