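; Flying-machine guard for the third boss stage that moves along a timeline path and fires blasts.
; Tick plays the timeline offset from its start location and requests fire regardless of range, throttled by a DoOnce with half-second reset.
; Damage at zero health sets Dead, destroys arrow, box and flipbook components, and plays an explosion, leaving the actor alive.
; Player height-tracking and range-gated attack events exist, but Tick calls neither.
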(event Custom|damage
  (params (DMG%20In :type Float%20%28single-precision%29))
  ;[1 1 1] damage guard
  (bind _output_get (Variables|Default|SetSecond_Stage_Guard_Health (- (Variables|Default|GetSecond_Stage_Guard_Health) DMG%20In)))
  (if (<= _output_get 0.0)
    (Variables|Default|SetDead true)
    (Utilities|FlowControl|Sequence
      (:then_0
        (Components|DestroyComponent (Variables|Default|GetFirst_Arrow)))
      (:then_1
        (Components|DestroyComponent (Variables|Default|GetFirst_Box)))
      (:then_2
        (Components|DestroyComponent (Variables|Default|Getmachine_guard_Flipbook)))
      (:then_3
        (Audio|PlaySound2D "/Game/Final_Project_Content/Sound_Music/SoundsCrate-SciFi-Explosion5__1_.SoundsCrate-SciFi-Explosion5__1_" 1.0 1.0 0.0 0 0)))))

(event Custom|Attack_Event
  ;[1 1 1] Event to shoot
  (bind _output_get (Variables|Default|Set3rd%20Boss%20Guard%20X%20Distance (- (.x (Transformation|GetActorLocation (Game|GetPlayerController 0))) (.x (Transformation|GetWorldLocation (Variables|Default|Getmachine_guard_Flipbook))))))
  (if (<= _output_get 3e+02)
    (Utilities|FlowControl|Sequence
      (:then_0
        (CallFunction|3rdStageGuardAttk)))))

(event Custom|3rd_Stage_Guard_Attk
  ;[1 1 1] Guard attk
  (Utilities|FlowControl|DoOnce false :!label _label
    (:Completed
      (Game|SpawnActorfromClass "/Game/Final_Project_Content/Blueprints/Attacks/BP_Blast_.BP_Blast__C" (Transformation|GetWorldTransform (Variables|Default|GetFirst_Arrow)) "Undefined" 0 0)
      (Utilities|FlowControl|Delay 0.5)
      (goto _label Reset))))

(event Custom|Move_Up_Down
  (bind _returnvalue (Transformation|GetActorLocation))
  (bind _returnvalue_2 (Game|GetPlayerCharacter 0))
  (bind _returnvalue_3 (Transformation|GetActorLocation))
  (bind _machine_guard_flipbook (Variables|Default|Getmachine_guard_Flipbook))
  (bind _returnvalue_4 (Transformation|GetActorLocation _returnvalue_2))
  (bind _returnvalue_5 (Transformation|GetWorldLocation _machine_guard_flipbook))
  (bind (_x _y _z) (Math|Vector|BreakVector _returnvalue))
  (bind (_x_2 _y_2 _z_2) (Math|Vector|BreakVector _returnvalue_3))
  ;[1 1 1] follows player on the z axis
  (Development|PrintString (Utilities|String|ToString(Float) (.z _returnvalue_4)))
  (Development|PrintString (Utilities|String|ToString(Float) (.z _returnvalue_5)))
  (bind _output_get (Variables|Default|Set3rd%20Boss%20Guard%20Z%20Distance (- (.z _returnvalue_4) (.z _returnvalue_5))))
  (if (> _output_get 5.0)
    (Transformation|SetActorLocation (Math|Vector|MakeVector _x_2 _y_2 (+ _z_2 1.5)) false false)
    (else
      (Transformation|SetActorLocation (Math|Vector|MakeVector _x _y (- _z 1.5)) false false))))

(event EventTick
  (params (DeltaSeconds :type Float%20%28single-precision%29))
  ;[1 1 1] Event Tick
  (Utilities|FlowControl|Sequence
    (:then_0
      (bind _newtrack (Timeline|Timeline_0 Play)
        (:Update
          (Transformation|SetActorLocation (+ _newtrack (Variables|Default|GetLocation%20of%20guard)) false false))))
    (:then_1
      (CallFunction|3rdStageGuardAttk))))

(event EventBeginPlay
  ;[1 1 1] Comment
  (Variables|Default|SetLocation%20of%20guard (Transformation|GetActorLocation))
  (Utilities|FlowControl|Delay 0.2)
  (Variables|Default|SetStart_Moving true))

(fn ConstructionScript)