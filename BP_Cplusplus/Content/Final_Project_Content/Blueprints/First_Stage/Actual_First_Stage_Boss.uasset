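; First-stage boss with a Paper2D sprite that chases the player along the X axis and shoots at them.
; Tick turns it to face the player in yaw and moves it a fixed step along +X, adding a catch-up step when the player is far ahead.
; An X-distance check triggers the attack, which spawns BP_Boss_Ammo at the Arrow, with a DoOnce and Delay cooldown.
; Z distance is computed, but the Z-follow movement is disconnected.
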(event OnComponentBeginOverlap(Capsule)
  (params (OverlappedComponent :type Primitive%20Component%20Object%20Reference) (OtherActor :type Actor%20Object%20Reference) (OtherComp :type Primitive%20Component%20Object%20Reference) (OtherBodyIndex :type Integer) (bFromSweep :type Boolean) (SweepResult :type Hit%20Result%20Structure%20%28by%20ref%29)))

(event Custom|First_Boss_Atck
  ;[1 1 1] Boss_Attack
  (Utilities|FlowControl|DoOnce false :!label _label
    (:Completed
      (Game|SpawnActorfromClass "/Game/Final_Project_Content/Blueprints/Attacks/BP_Boss_Ammo.BP_Boss_Ammo_C" (Transformation|GetWorldTransform (Variables|Default|GetArrow)) "Undefined" 0 0)
      (Utilities|FlowControl|Delay 4.0)
      (goto _label Reset))))

(event EventTick
  (params (DeltaSeconds :type Float%20%28single-precision%29))
  (bind _returnvalue (Transformation|GetActorLocation))
  (bind _returnvalue_2 (Transformation|GetActorLocation))
  (bind _returnvalue_3 (Transformation|GetActorLocation))
  (bind (_x _y _z) (Math|Vector|BreakVector _returnvalue_2))
  (bind (_x_2 _y_2 _z_2) (Math|Vector|BreakVector _returnvalue_3))
  (Utilities|FlowControl|Sequence
    (:then_0
      (Transformation|SetActorRotation (Math|Rotator|MakeRotator 0.0 0.0 (.yaw (Math|Rotator|FindLookatRotation (Transformation|GetActorLocation) (Transformation|GetActorLocation (Game|GetPlayerCharacter 0)))))))
    (:then_1
      (bind _output_get (Variables|Default|SetFirst_Boss_X_Distance (- (.x (Transformation|GetActorLocation (Game|GetPlayerController 0))) (.x (Transformation|GetWorldLocation (Variables|Default|GetPaperSprite))))))
      (if (<= _output_get 2e+02)
        (CallFunction|FirstBossAtck)))
    (:then_2
      (Variables|Default|SetActorX (.x _returnvalue)))
    (:then_3
      (Variables|Default|SetActorY (.y _returnvalue)))
    (:then_4
      (Variables|Default|SetActorZ (.z _returnvalue)))
    (:then_5
      (if (Math|Float|InRange(Float) (Variables|Default|GetFirst_Boss_X_Distance) 0.0 4e+02)
        (Transformation|SetActorLocation (Math|Vector|MakeVector (Variables|Default|GetActorX) (Variables|Default|GetActorY) (Variables|Default|GetActorZ)) false false)))
    (:then_6
      ;[1 1 1] Boss Moving on X Axis
      (Transformation|SetActorLocation (Math|Vector|MakeVector (+ _x 1.2) _y _z) false false))
    (:then_7
      ;[1 1 1] Boss Moving on Z Axis
      (bind _output_get_2 (Variables|Default|SetFirst_Boss_Z_Distance (- (.z (Transformation|GetActorLocation (Game|GetPlayerCharacter 0))) (.z (Transformation|GetWorldLocation (Variables|Default|GetPaperSprite)))))))
    (:then_8
      ;[1 1 1] If distance between player and boss and over certain amount boss will speed up to catch up to player
      (bind _output_get_3 (Variables|Default|SetFirst_Boss_X_Distance (- (.x (Transformation|GetActorLocation (Game|GetPlayerCharacter 0))) (.x (Transformation|GetWorldLocation (Variables|Default|GetPaperSprite))))))
      (if (>= _output_get_3 4e+02)
        (Transformation|SetActorLocation (Math|Vector|MakeVector (+ _x_2 1.0) _y_2 _z_2) false false)))))

(fn ConstructionScript)